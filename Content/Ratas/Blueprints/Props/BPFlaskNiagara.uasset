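; BPFlaskNiagara is a flask's area-effect actor that pairs a Niagara effect with a damaging sphere and destroys itself when the effect finishes.
; Foe-tagged components entering the sphere trigger a one-off hit on their RatasCharacterFoe owner.
; A Tick countdown periodically applies a weaker hit to the owners of overlapping Foe or Player components, so the area also hurts players.
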(event OnComponentBeginOverlap(Sphere)
  (params (OverlappedComponent :type Primitive%20Component%20Object%20Reference) (OtherActor :type Actor%20Object%20Reference) (OtherComp :type Primitive%20Component%20Object%20Reference) (OtherBodyIndex :type Integer) (bFromSweep :type Boolean) (SweepResult :type Hit%20Result%20Structure%20%28by%20ref%29))
  (if (Components|ComponentHasTag OtherComp "Foe")
    (bind _asratas_character_foe (Utilities|Casting|CastToRatasCharacterFoe OtherActor))
    (Class|RatasCharacterFoe|GetHit _asratas_character_foe 1.0)))

(event OnSystemFinished(Niagara)
  (params (PSystem :type Niagara%20Component%20Object%20Reference))
  (Actor|DestroyActor))

(event EventBeginPlay)

(event Collision|EventActorBeginOverlap
  (params (OtherActor :type Actor%20Object%20Reference)))

(event EventTick
  (params (DeltaSeconds :type Float%20%28single-precision%29))
  (bind _output_get (Variables|Default|SetDamageTimer (- (Variables|Default|GetDamageTimer) DeltaSeconds)))
  (if (<= _output_get 0.0)
    (for _array_element (Class|PrimitiveComponent|GetOverlappingComponents (Variables|Default|GetSphere))
      (if (or (Components|ComponentHasTag _array_element "Foe") (Components|ComponentHasTag _array_element "Player"))
        (bind _asratas_character (Utilities|Casting|CastToRatasCharacter (Components|GetOwner _array_element)))
        (Class|RatasCharacter|GetHit _asratas_character 0.5)))
    (Variables|Default|SetDamageTimer (Variables|Default|GetDamageTimerMax))))

(fn ConstructionScript)