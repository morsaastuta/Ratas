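; BP_Shotgun is a shotgun weapon that fires a spread of Bullet actors aimed at targets tagged "Foe".
; Trigger spawns a burst of pellets at the Barrel with random pitch and yaw offsets, passing in Damage, Impulse as speed and a short despawn timer.
; It caches the mesh's ABP_Shotgun instance on BeginPlay, flags Shooting on each trigger pull and copies Reloading to it every Tick.
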(event EventTick
  (params (DeltaSeconds :type Float%20%28single-precision%29))
  (Variables|/Game/Ratas/Blueprints/Weapons/ABP_Shotgun.ABP_Shotgun_C|SetReloading (Variables|Default|GetABP) (Variables|Default|GetReloading)))

(event EventBeginPlay
  (CallFunction|CastAnimationBlueprint))

(event EventTrigger
  (bind _barrel (Variables|Default|GetBarrel))
  (bind _returnvalue (Transformation|GetWorldTransform _barrel))
  (Variables|/Game/Ratas/Blueprints/Weapons/ABP_Shotgun.ABP_Shotgun_C|SetShooting (Variables|Default|GetABP) true)
  (for _index (range 0 11)
    (Game|SpawnActorfromClass (Variables|Default|GetBullet) (Math|Transform|MakeTransform (.location _returnvalue) (Math|Rotator|MakeRotator (.roll (.rotation _returnvalue)) (+ (.pitch (.rotation _returnvalue)) (- (* (Math|Random|RandomFloat) 4e+01) 2e+01)) (+ (.yaw (.rotation _returnvalue)) (- (* (Math|Random|RandomFloat) 4e+01) 2e+01))) (.scale _returnvalue)) "Undefined" "MultiplyWithRoot" 0 (Variables|Default|GetDamage) (Variables|Default|GetImpulse) 2.0 "Foe" 0)))

(fn ConstructionScript)

(fn CastAnimationBlueprint
  (bind _asabp_shotgun (Utilities|Casting|CastToABP_Shotgun (Components|SkeletalMesh|GetAnimInstance (Variables|Character|GetMesh))))
  (Variables|Default|SetABP _asabp_shotgun))