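; Enemy Blueprint for the RataGorda foe, which turns toward a detected player and advances while alive.
; Each tick it fetches its Animation Blueprint, passes it the targeting state, shoot origin and an axis-offset head rotation.
; Interpolated look-at yaw from the head bone drives Look and actor rotation, followed by a Move call.
; AfterChecks sets the animation's dead flag from Health, which halts this behavior.
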(event Custom|CastAnimationBlueprint
  (bind _asabp_foe_rata_gorda (Utilities|Casting|CastToABP_Foe_RataGorda (Components|SkeletalMesh|GetAnimInstance (Variables|Character|GetMesh))))
  (Variables|Default|SetABP _asabp_foe_rata_gorda))

(event EventBeginPlay)

(event Collision|EventActorBeginOverlap
  (params (OtherActor :type Actor%20Object%20Reference)))

(event EventAfterChecks
  (Variables|/Game/Ratas/FBX/FatRat/ABP_Foe_RataGorda.ABP_Foe_RataGorda_C|SetIsDead (Variables|Default|GetABP) (<= (Variables|Default|GetHealth) 0)))

(event EventTick
  (params (DeltaSeconds :type Float%20%28single-precision%29))
  (bind _targetlocation (Variables|Default|GetTargetLocation))
  (bind _mesh (Variables|Character|GetMesh))
  (bind _returnvalue (Transformation|GetBoneTransform _mesh "head_001" "RTS_World"))
  (bind _returnvalue_2 (Math|Rotator|FindLookatRotation (.location _returnvalue) _targetlocation))
  (bind _returnvalue_3 (Math|Interpolation|RInterpTo (Math|Rotator|MakeRotator 0.0 0.0 (.yaw (.rotation _returnvalue))) (Math|Rotator|MakeRotator 0.0 0.0 (.yaw _returnvalue_2)) 0.5 0.0))
  (CallFunction|CastAnimationBlueprint)
  (if (not (Variables|/Game/Ratas/FBX/FatRat/ABP_Foe_RataGorda.ABP_Foe_RataGorda_C|GetIsDead (Variables|Default|GetABP)))
    (bind _returnvalue_4 (Class|RatasCharacterFoe|DetectPlayer))
    (bind _output_get (Variables|/Game/Ratas/FBX/FatRat/ABP_Foe_RataGorda.ABP_Foe_RataGorda_C|SetTargeted (Variables|Default|GetABP) _returnvalue_4))
    (if _output_get
      (Variables|/Game/Ratas/FBX/FatRat/ABP_Foe_RataGorda.ABP_Foe_RataGorda_C|SetShootOrigin (Variables|Default|GetABP) (Transformation|GetActorTransform))
      (Variables|/Game/Ratas/FBX/FatRat/ABP_Foe_RataGorda.ABP_Foe_RataGorda_C|SetRotation%20Foe (Variables|Default|GetABP) (Math|Interpolation|RInterpTo (Math|Rotator|MakeRotator (+ (.roll (.rotation _returnvalue)) -9e+01) (+ (.pitch (.rotation _returnvalue)) 1.8e+02) (+ (.yaw (.rotation _returnvalue)) 9e+01)) (Math|Rotator|MakeRotator (+ (.roll _returnvalue_2) -9e+01) (+ (.pitch _returnvalue_2) 1.8e+02) (+ (.yaw _returnvalue_2) 9e+01)) 0.5 0.0))
      (Class|RatasCharacter|Look (Math|Rotator|GetRotationXVector _returnvalue_3))
      (Transformation|SetActorRotation _returnvalue_3)
      (bind _output_get_2 (Variables|Default|SetForward "0.000000,0.100000,0.000000"))
      (Class|RatasCharacter|Move _output_get_2))))

(fn ConstructionScript)