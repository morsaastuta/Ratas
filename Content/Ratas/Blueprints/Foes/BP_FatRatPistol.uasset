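; Pistol-wielding fat rat enemy that chases and aims at the player, driving its state through ABP_FatRatPistol.
; Each tick while alive, a player in EngageRange sets Shootable and gets ShootPoint aimed, with its transform passed to the AnimBP as ShootOrigin.
; Otherwise, a player in DetectionRange sets Targeted and the rat moves forward.
; Turning interpolates yaw from the head bone toward the target; AfterChecks flags death at zero health.
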(event EventBeginPlay
  (CallFunction|CastAnimationBlueprint))

(event EventAfterChecks
  (Variables|/Game/Ratas/Blueprints/Foes/ABP_FatRatPistol.ABP_FatRatPistol_C|SetIsDead (Variables|Default|GetABP) (<= (Variables|Default|GetHealth) 0.0)))

(event EventTick
  (params (DeltaSeconds :type Float%20%28single-precision%29))
  (if (not (Variables|/Game/Ratas/Blueprints/Foes/ABP_FatRatPistol.ABP_FatRatPistol_C|GetIsDead (Variables|Default|GetABP)))
    (bind (_player _returnvalue) (Class|RatasCharacterFoe|CheckPlayer (Variables|Default|GetEngageRange)))
    (bind _output_get (Variables|/Game/Ratas/Blueprints/Foes/ABP_FatRatPistol.ABP_FatRatPistol_C|SetShootable (Variables|Default|GetABP) _returnvalue))
    (if _output_get
      (Class|RatasCharacterFoe|Lookat (Transformation|GetActorLocation _player))
      (CallFunction|LookatPlayer)
      (Transformation|SetWorldRotation (Variables|Default|GetShootPoint) (Math|Rotator|FindLookatRotation (Transformation|GetWorldLocation (Variables|Default|GetShootPoint)) (Variables|Default|GetTargetLocation)) false false)
      (Variables|/Game/Ratas/Blueprints/Foes/ABP_FatRatPistol.ABP_FatRatPistol_C|SetShootOrigin (Variables|Default|GetABP) (Transformation|GetWorldTransform (Variables|Default|GetShootPoint)))
      (else
        (bind (_player_2 _returnvalue_2) (Class|RatasCharacterFoe|CheckPlayer (Variables|Default|GetDetectionRange)))
        (bind _output_get_2 (Variables|/Game/Ratas/Blueprints/Foes/ABP_FatRatPistol.ABP_FatRatPistol_C|SetTargeted (Variables|Default|GetABP) _returnvalue_2))
        (if _output_get_2
          (Class|RatasCharacterFoe|Lookat (Transformation|GetActorLocation _player_2))
          (CallFunction|LookatPlayer)
          (Class|RatasCharacter|Move (Variables|Default|GetForward)))))))

(fn ConstructionScript)

(fn LookatPlayer
  (bind _mesh (Variables|Character|GetMesh))
  (bind _returnvalue (Transformation|GetBoneTransform _mesh "head_001" "RTS_World"))
  (Transformation|SetActorRotation (Math|Interpolation|RInterpTo (Math|Rotator|MakeRotator 0.0 0.0 (.yaw (.rotation _returnvalue))) (Math|Rotator|MakeRotator 0.0 0.0 (.yaw (Math|Rotator|FindLookatRotation (.location _returnvalue) (Variables|Default|GetTargetLocation)))) 0.5 0.0)))

(fn CastAnimationBlueprint
  (bind _asabp_fat_rat_pistol (Utilities|Casting|CastToABP_FatRatPistol (Components|SkeletalMesh|GetAnimInstance (Variables|Character|GetMesh))))
  (Variables|Default|SetABP _asabp_fat_rat_pistol))