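; BP_Foe_SkinnyRat_Unarmed is an unarmed skinny rat enemy that chases and punches the player.
; Each tick while alive, range checks set animation blueprint flags: within engage range it faces the player and can punch, within detection range it turns by head-bone yaw and advances.
; Hit collision overlaps follow the attacking flag while engaged, dealing one hit when CanHit allows, then clearing it.
; Depleted health marks it dead.
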(event OnComponentBeginOverlap(HitCollision)
  (params (OverlappedComponent :type Primitive%20Component%20Object%20Reference) (OtherActor :type Actor%20Object%20Reference) (OtherComp :type Primitive%20Component%20Object%20Reference) (OtherBodyIndex :type Integer) (bFromSweep :type Boolean) (SweepResult :type Hit%20Result%20Structure%20%28by%20ref%29))
  (if (Variables|/Game/Ratas/Blueprints/Foes/ABP_SkinnyRat.ABP_SkinnyRat_C|GetCanHit (Variables|Default|GetABP))
    (bind (_player _returnvalue) (Class|RatasCharacterFoe|CheckPlayer (Variables|Default|GetHitCollision)))
    (if _returnvalue
      (Variables|/Game/Ratas/Blueprints/Foes/ABP_SkinnyRat.ABP_SkinnyRat_C|SetCanHit (Variables|Default|GetABP) false)
      (Class|RatasCharacterPlayer|GetHit _player 1)
      (Development|PrintString "Hello"))))

(event EventBeginPlay
  (CallFunction|CastAnimationBlueprint))

(event EventAfterChecks
  (Variables|/Game/Ratas/Blueprints/Foes/ABP_SkinnyRat.ABP_SkinnyRat_C|SetIsDead (Variables|Default|GetABP) (<= (Variables|Default|GetHealth) 0)))

(event EventTick
  (params (DeltaSeconds :type Float%20%28single-precision%29))
  (if (not (Variables|/Game/Ratas/Blueprints/Foes/ABP_SkinnyRat.ABP_SkinnyRat_C|GetIsDead (Variables|Default|GetABP)))
    (bind (_player _returnvalue) (Class|RatasCharacterFoe|CheckPlayer (Variables|Default|GetEngageRange)))
    (bind _output_get (Variables|/Game/Ratas/Blueprints/Foes/ABP_SkinnyRat.ABP_SkinnyRat_C|SetPunchable (Variables|Default|GetABP) _returnvalue))
    (if _output_get
      (Class|RatasCharacterFoe|Lookat (Transformation|GetActorLocation _player))
      (Variables|/Script/Engine.PrimitiveComponent|SetbGenerateOverlapEvents (Variables|Default|GetHitCollision) (Variables|/Game/Ratas/Blueprints/Foes/ABP_SkinnyRat.ABP_SkinnyRat_C|GetAttacking (Variables|Default|GetABP)))
      (else
        (bind (_player_2 _returnvalue_2) (Class|RatasCharacterFoe|CheckPlayer (Variables|Default|GetDetectionRange)))
        (bind _output_get_2 (Variables|/Game/Ratas/Blueprints/Foes/ABP_SkinnyRat.ABP_SkinnyRat_C|SetTargeted (Variables|Default|GetABP) _returnvalue_2))
        (if _output_get_2
          (Class|RatasCharacterFoe|Lookat (Transformation|GetActorLocation _player_2))
          (CallFunction|LookatPlayer)
          (Class|RatasCharacter|Move (Variables|Default|GetForward)))))))

(fn ConstructionScript)

(fn LookatPlayer
  (bind _mesh (Variables|Character|GetMesh))
  (bind _returnvalue (Transformation|GetBoneTransform _mesh "head_001" "RTS_World"))
  (Transformation|SetActorRotation (Math|Interpolation|RInterpTo (Math|Rotator|MakeRotator 0.0 0.0 (.yaw (.rotation _returnvalue))) (Math|Rotator|MakeRotator 0.0 0.0 (.yaw (Math|Rotator|FindLookatRotation (.location _returnvalue) (Variables|Default|GetTargetLocation)))) 0.5 0.0)))

(fn CastAnimationBlueprint
  (bind _asabp_skinny_rat_unarmed (Utilities|Casting|CastToABP_SkinnyRat (Components|SkeletalMesh|GetAnimInstance (Variables|Character|GetMesh))))
  (Variables|Default|SetABP _asabp_skinny_rat_unarmed))